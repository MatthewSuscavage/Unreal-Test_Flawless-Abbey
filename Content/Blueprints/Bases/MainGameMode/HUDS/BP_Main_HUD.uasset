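; Main game HUD that creates the general HUD and inventories widgets on BeginPlay and relays interaction messages and inventory updates to them.
; Inventory events either show a given inventory in a viewport alongside the player's main inventory, or toggle the player's inventory alone.
; Toggling flips widget visibility, input mode and mouse cursor, and adds or removes the UI Enhanced Input mapping context.
; Game-pausing nodes are present but unconnected, so play continues while inventories are open.
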(event EventBeginPlay
  (Utilities|FlowControl|Sequence
    (:then_0
      ;[0.15 0.15 0.15 0.5] Focusing on the Game
      (Input|SetInputModeGameOnly (Game|Player|GetOwningPlayerController) false))
    (:then_1
      ;[0.15 0.15 0.15 0.5] Creating and adding the hud to Viewport
      (bind _returnvalue (UserInterface|CreateWidget "/Game/Widgets/HUD/WB_HUD.WB_HUD_C" (Game|Player|GetOwningPlayerController)))
      (bind _output_get (Variables|Default|SetHUD_WB _returnvalue))
      (UserInterface|Viewport|AddtoViewport _output_get 0))
    (:then_2
      ;[0.15 0.15 0.15 0.5] Creating inventories widget
      (bind _returnvalue_2 (UserInterface|CreateWidget "/Game/Widgets/Inventory/WB_Inventories.WB_Inventories_C" (Game|Player|GetOwningPlayerController)))
      (bind _output_get_2 (Variables|Default|SetInventories_HUD _returnvalue_2))
      (UserInterface|Viewport|AddtoViewport _output_get_2 0))))

(event EventShowInteractionMessage
  (params (Interaction_Message :type Text))
  ;[0.15 0.15 0.15 0.5] Shows interaction message
  (Default|ShowInteractionMessage (Variables|Default|GetHUD_WB) Interaction_Message))

(event EventHideInteractionMessage
  ;[0.15 0.15 0.15 0.5] Hides interaction message
  (Default|HideInteracitonMessage (Variables|Default|GetHUD_WB)))

(event EventSetMainPlayerInventory
  (params (Inventory :type BPC%20Inventory%20Object%20Reference))
  ;[0.15 0.15 0.15 0.5] Setting main player inventory
  (bind _inventories_hud (Variables|Default|GetInventories_HUD)
    (:then
      (Default|SetMainPlayerInventory _inventories_hud Inventory))
    (:else)))

(event EventUpdateMainPlayerSlots
  ;[0.15 0.15 0.15 0.5] Update main player slots
  (Default|UpdateMainPlayerInventory (Variables|Default|GetInventories_HUD)))

(event EventTogglePlayerInventory
  (bind _inventories_hud (Variables|Default|GetInventories_HUD))
  ;[0.15 0.15 0.15 0.5] Toggles player main inventory
  (bind _visible_ (CallFunction|ToggleWidgetVisibility _inventories_hud))
  (CallFunction|ToggleUIInputMapping _visible_)
  (if _visible_
    (Default|UpdateMainPlayerInventory _inventories_hud)
    (else
      (Default|HideViewport _inventories_hud))))

(event EventUpdateViewportSlots
  ;[0.15 0.15 0.15 0.5] Update Viewport Inventory Slots
  (Default|UpdateViewport (Variables|Default|GetInventories_HUD)))

(event EventToggleViewport
  (params (Inventory :type BPC%20Inventory%20Object%20Reference) (Inventory%20Name :type Text))
  (bind _inventories_hud (Variables|Default|GetInventories_HUD))
  ;[0.15 0.15 0.15 0.5] Showing Viewport
  (bind _visible_ (CallFunction|ToggleWidgetVisibility _inventories_hud))
  (CallFunction|ToggleUIInputMapping _visible_)
  (if _visible_
    (Default|ShowViewport _inventories_hud Inventory Inventory%20Name)
    (Default|UpdateViewport _inventories_hud)
    (Default|UpdateMainPlayerInventory _inventories_hud)
    (else
      (Default|HideViewport _inventories_hud))))

(fn ConstructionScript)

(fn ToggleWidgetVisibility
  (params (Widget :type User%20Widget%20Object%20Reference))
  (bind _returnvalue (Game|Player|GetOwningPlayerController))
  (bind _returnvalue_2 (Game|Player|GetOwningPlayerController))
  (if (Widget|IsVisible Widget)
    (Widget|SetVisibility Widget "Collapsed")
    (Input|SetInputModeGameOnly _returnvalue_2 false)
    (Variables|/Script/Engine.PlayerController|SetbShowMouseCursor _returnvalue_2 false)
    (return false)
    (else
      (Widget|SetVisibility Widget "Visible")
      (Input|SetInputModeGameandUI _returnvalue Widget "DoNotLock" true false)
      (Variables|/Script/Engine.PlayerController|SetbShowMouseCursor _returnvalue true)
      (return true))))

(fn ToggleUIInputMapping
  (params (Visible? :type Boolean))
  (bind _returnvalue (Game|Player|GetOwningPlayerController))
  (bind _returnvalue_2 (Game|Player|GetOwningPlayerController))
  (bind _returnvalue_3 (PlayerController|LocalPlayerSubsystems|GetEnhancedInputLocalPlayerSubsystem _returnvalue))
  (bind _returnvalue_4 (PlayerController|LocalPlayerSubsystems|GetEnhancedInputLocalPlayerSubsystem _returnvalue_2))
  (if Visible?
    (Utilities|IsValid _returnvalue_4
      (:Is%20Valid
        (Input|AddMappingContext _returnvalue_4 "/Game/Input/Default/UI/IMC_UI.IMC_UI" 0 "(bIgnoreAllPressedKeysUntilRelease=True,bForceImmediately=False,bNotifyUserSettings=False)")))
    (else
      (Utilities|IsValid _returnvalue_3
        (:Is%20Valid
          (Input|RemoveMappingContext _returnvalue_3 "/Game/Input/Default/UI/IMC_UI.IMC_UI" "(bIgnoreAllPressedKeysUntilRelease=True,bForceImmediately=False,bNotifyUserSettings=False)"))))))