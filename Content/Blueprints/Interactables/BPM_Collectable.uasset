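; BPM_Collectable is an interactable pickup that gives an item to the player's inventory.
; On Interact, it sends the ItemInfo row name and Amount to player character 0 through an AddItemToInventory message.
; It subtracts the returned count from Amount and destroys itself when nothing remains, so a partial pickup leaves the remainder in the world.
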(event EventBeginPlay
  (|CallParentFunction) ; This node is disabled and will not be called.\nDrag off pins to build functionality.
)

(event Collision|EventActorBeginOverlap
  (params (OtherActor :type Actor%20Object%20Reference))
  (|CallParentFunction OtherActor) ; This node is disabled and will not be called.\nDrag off pins to build functionality.
)

(event EventTick
  (params (DeltaSeconds :type Float%20%28single-precision%29))
  (|CallParentFunction DeltaSeconds) ; This node is disabled and will not be called.\nDrag off pins to build functionality.
)

(event EventInteract
  (bind _items_added (Class|BPIPlayer|AddItemtoInventory(Message) (Game|GetPlayerCharacter 0) (.rowname (Variables|Default|GetItem_Info)) (Variables|Default|GetAmount)))
  (if (<= (- (Variables|Default|GetAmount) _items_added) 0)
    (Actor|DestroyActor)
    (else
      (Variables|Default|SetAmount (- (Variables|Default|GetAmount) _items_added)))))

(fn ConstructionScript
  (|CallParentFunction))